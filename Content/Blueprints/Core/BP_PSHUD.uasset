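; HUD Blueprint that shows interaction hints and the end-of-game screen.
; On BeginPlay it binds to the OnGameEnded dispatcher of BP_PSGameState.
; ShowEndGameScreen adds a WBP_GameEnded widget that is given the win result.
; OnInteractTriggerChanged removes the current action hint and, if the new trigger is valid, creates a WBP_ActionHint for it.
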(event `self.ReceiveBeginPlay`
  (bind _asbp_psgame_state (cast `/Game/Blueprints/Core/BP_PSGameState` (`GameplayStatics.GetGameState`)))
  (add `PSGameStateBase.OnGameEnded` _asbp_psgame_state (`|CreateDelegate` :!event `Show End Game Screen`)))

(event `Show End Game Screen`
  (params (bWin :type Boolean))
  (bind _returnvalue (`|CreateWidget` "/Game/Widgets/HUD/WBP_GameEnded.WBP_GameEnded_C" null bWin))
  (`UserWidget.AddToViewport` _returnvalue 0))

(fn `OnInteractTriggerChanged`
  (params (OldTrigger :type "PSInteractTriggerComponent Object Reference") (NewTrigger :type "PSInteractTriggerComponent Object Reference"))
  (`/Engine/EditorBlueprintResources/StandardMacros.IsValid` (`self.Action Hint`)
    (:`Is Valid`
      (`Widget.RemoveFromParent` (`self.Action Hint`)))
    (:`Is Not Valid`
      _))
  (`/Engine/EditorBlueprintResources/StandardMacros.IsValid` (`local.NewTrigger`)
    (:`Is Valid`
      (bind _returnvalue (`|CreateWidget` "/Game/Widgets/HUD/WBP_ActionHint.WBP_ActionHint_C" null (`local.NewTrigger`)))
      (bind _output_get (set `self.Action Hint` _returnvalue))
      (`UserWidget.AddToViewport` _output_get 0))))

(fn `UserConstructionScript`)