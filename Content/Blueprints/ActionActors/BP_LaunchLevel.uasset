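; An action actor that opens another level when its interact trigger fires.
; On BeginPlay it looks up the level by name and, if found, passes the level struct to its WBP_LaunchLevel widget.
; It also binds to activity changes, switching the cube between blue and gray materials to show active state.
; The trigger calls TryPerformAction, and PerformAction opens the stored level by object reference.
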(event `self.ReceiveBeginPlay`
  (bind (_foundlevel _returnvalue) (`PSLevelSettings.FindLevel` (`self.Level Name`)))
  (if _returnvalue
    (set `self.Level Struct` _foundlevel)
    (add `self.OnActivityChanged` (`|CreateDelegate` :!event `On Activity Changed`))
    (`self.On Activity Changed` (`self.bIsActive`))
    (bind _aswbp_launch_level (cast `/Game/Widgets/WBP_LaunchLevel` (`WidgetComponent.GetWidget` (`self.Widget`))))
    (`/Game/Widgets/WBP_LaunchLevel.Set Level` _aswbp_launch_level (`self.Level Struct`))))

(event `On Activity Changed` :!signature `self.OnActivityChanged`
  (params (bNewActive :type Boolean))
  (`PrimitiveComponent.SetMaterial` (`self.Cube`) 0 (select `bool` bNewActive :`false` "/Game/Materials/Plastic/MI_Plastic_Gray.MI_Plastic_Gray" :`true` "/Game/Materials/Plastic/MI_Plastic_Blue.MI_Plastic_Blue" :!type "MaterialInterface Object Reference")))

(event `self.PSInteractTrigger.OnTriggerBegin`
  (params (TriggerSource :type "PSTriggerSource Interface") (TriggerComponent :type "PSTriggerComponent Object Reference"))
  (`self.TryPerformAction` TriggerSource))

(event `self.PerformAction`
  (params (TriggerSource :type "PSTriggerSource Interface (by ref)"))
  (`GameplayStatics.OpenLevelBySoftObjectPtr` (`.LevelObject` (break `PSLevel` (`self.Level Struct`)))))

(fn `UserConstructionScript`)